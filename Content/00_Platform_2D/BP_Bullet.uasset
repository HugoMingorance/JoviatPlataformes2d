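; BP_Bullet is a projectile actor in the 2D platformer folder that flies straight and explodes on contact.
; Tick moves it along its forward vector by Speed scaled by delta time, without sweeping, and BeginPlay sets a timer event to destroy it.
; On overlap it prints the other actor's name, then spawns an explosion, plays a sound and destroys itself unless that name contains "Camera".
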(event `self.ReceiveBeginPlay`
  (`KismetSystemLibrary.K2_SetTimerDelegate` (delegate `Destroy Bullet`)))

(event `Destroy Bullet`
  (`self.K2_DestroyActor`))

(event `self.ReceiveTick`
  (params (DeltaSeconds :type "Float (single-precision)"))
  (`self.K2_SetActorLocation` (+ (`self.K2_GetActorLocation`) (* (* DeltaSeconds (`self.speed`)) (`self.GetActorForwardVector`)))))

(event `self.ReceiveActorBeginOverlap`
  (params (OtherActor :type "Actor Object Reference"))
  (bind _returnvalue (`KismetSystemLibrary.GetDisplayName` OtherActor))
  (`KismetSystemLibrary.PrintString` "Collided with:")
  (`KismetSystemLibrary.PrintString` _returnvalue)
  (if (not (`KismetStringLibrary.Contains` _returnvalue "Camera"))
    (`GameplayStatics.SpawnEmitterAtLocation` "/Game/StarterContent/Particles/P_Explosion.P_Explosion" (`self.K2_GetActorLocation`))
    (`GameplayStatics.PlaySound2D` "/Game/StarterContent/Audio/Explosion02.Explosion02" 1.0 1.0 0.0 null null)
    (`self.K2_DestroyActor`)))

(fn `UserConstructionScript`)